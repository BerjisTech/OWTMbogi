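; OilStamps is an oil patch hazard actor that jolts vehicles driving over it.
; When a VehicleBasePawn overlaps its static mesh, it adds an impulse to the vehicle's mesh along the forward axis, randomly forward or backward with random strength, plus the negligible normalized velocity.
; The impulse is applied at the world origin rather than at the vehicle, so any spin it causes depends on where the vehicle is.
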(event OnComponentBeginOverlap(StaticMesh)
  (params (OverlappedComponent :type Primitive%20Component%20Object%20Reference) (OtherActor :type Actor%20Object%20Reference) (OtherComp :type Primitive%20Component%20Object%20Reference) (OtherBodyIndex :type Integer) (bFromSweep :type Boolean) (SweepResult :type Hit%20Result%20Structure%20%28by%20ref%29))
  (bind _returnvalue (Math|Random|RandomFloatinRange -1.5e+03 -8e+02))
  (if (Class|GameplayStatics|ObjectIsA OtherActor "/openWorldTemplate/vehicles/blueprint/VehicleBasePawn.VehicleBasePawn_C")
    (Physics|AddImpulseatLocation (Variables|/Script/ChaosVehicles.WheeledVehiclePawn|GetMesh (.AsVehicle%20Base%20Pawn (Utilities|Casting|CastToVehicleBasePawn OtherActor))) (+ (Math|Vector|Normalize (Transformation|GetVelocity OtherActor)) (* (Transformation|GetActorForwardVector OtherActor) (Math|Float|SelectFloat _returnvalue (Math|Float|Absolute(Float) _returnvalue) (Math|Random|RandomBool)))) "0, 0, 0" "None")))

(event EventBeginPlay)

(event EventTick
  (params (DeltaSeconds :type Float%20%28single-precision%29)))

(event Collision|EventActorBeginOverlap
  (params (OtherActor :type Actor%20Object%20Reference)))

(fn ConstructionScript)