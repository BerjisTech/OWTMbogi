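; Timer actor that starts an on-screen elapsed-time readout when something begins overlapping its Box component.
; The overlap calls a custom event that stores the current time as StartTime, then enters an endless loop built on a tiny Delay rather than Tick.
; Each pass prints hours, minutes and seconds since StartTime through a keyed Print String, with no stop condition or overlap filter.
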(event OnComponentBeginOverlap(Box)
  (params (OverlappedComponent :type Primitive%20Component%20Object%20Reference) (OtherActor :type Actor%20Object%20Reference) (OtherComp :type Primitive%20Component%20Object%20Reference) (OtherBodyIndex :type Integer) (bFromSweep :type Boolean) (SweepResult :type Hit%20Result%20Structure%20%28by%20ref%29))
  (CallFunction|StartTimer))

(event Custom|startTimer
  (Variables|Default|SetstartTime (Math|DateTime|Now))
  (Development|PrintString (Utilities|String|Append "Time " ":" (Utilities|String|ToString(Integer) (.hours (- (Math|DateTime|Now) (Variables|Default|GetstartTime)))) ":" (Utilities|String|ToString(Integer) (.minutes (- (Math|DateTime|Now) (Variables|Default|GetstartTime)))) ":" (Utilities|String|ToString(Integer) (.seconds (- (Math|DateTime|Now) (Variables|Default|GetstartTime))))) true true "(R=0.000000,G=0.660000,B=1.000000,A=1.000000)" 2.0 "timer" :!label _label)
  (Utilities|FlowControl|Delay 2e-06)
  (goto _label))

(event EventBeginPlay)

(event Collision|EventActorBeginOverlap
  (params (OtherActor :type Actor%20Object%20Reference)))

(event EventTick
  (params (DeltaSeconds :type Float%20%28single-precision%29)))

(fn ConstructionScript)