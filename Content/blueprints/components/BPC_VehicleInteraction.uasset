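; Vehicle interaction component that handles a driver taking control of a vehicle and handing it back.
; PossessVehicle stores the vehicle and driver, then has the driver's controller possess the vehicle.
; IA_Interact or possesDriver adds BPC_PlayerInteraction to the driver and sends it a possess message with both references.
; The driver is then teleported to a fixed offset from the vehicle.
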(event Custom|possesDriver
  (bind _vehicle (Variables|Default|GetVehicle))
  (bind _driver (Variables|Default|GetDriver))
  (Utilities|AddInteractionComponent (Variables|Default|GetDriver) "/openWorldTemplate/blueprints/components/BPC_PlayerInteraction.BPC_PlayerInteraction_C")
  (Class|BPIWorldInteraction|PossessVehicle(Message) (Actor|GetComponentbyClass (Variables|Default|GetDriver) "/openWorldTemplate/blueprints/components/BPC_PlayerInteraction.BPC_PlayerInteraction_C") true false (Utilities|ResolveSoftReference _vehicle) (Utilities|ResolveSoftReference _driver))
  (Transformation|SetActorLocation _driver (+ (Transformation|GetActorLocation _vehicle) 4e+02) false true))

(event Input|EnhancedActionEvents|EnhancedInputActionIA_Interact
  (params (ActionValue :type Boolean) (ElapsedSeconds :type Float%20%28double-precision%29) (TriggeredSeconds :type Float%20%28double-precision%29) (InputAction :type Input%20Action%20Object%20Reference :default "/openWorldTemplate/blueprints/Input/Actions/IA_Interact.IA_Interact"))
  (bind _vehicle (Variables|Default|GetVehicle))
  (bind _driver (Variables|Default|GetDriver))
  (:Started
    (Utilities|AddInteractionComponent (Variables|Default|GetDriver) "/openWorldTemplate/blueprints/components/BPC_PlayerInteraction.BPC_PlayerInteraction_C")
    (Class|BPIWorldInteraction|PossessVehicle(Message) (Actor|GetComponentbyClass (Variables|Default|GetDriver) "/openWorldTemplate/blueprints/components/BPC_PlayerInteraction.BPC_PlayerInteraction_C") true false (Utilities|ResolveSoftReference _vehicle) (Utilities|ResolveSoftReference _driver))
    (Transformation|SetActorLocation _driver (+ (Transformation|GetActorLocation _vehicle) 4e+02) false true)))

(event EventBeginPlay)

(event EventTick
  (params (DeltaSeconds :type Float%20%28single-precision%29)))

(event EventPossessVehicle
  (params (possess :type Boolean) (is_npc :type Boolean) (vehicle :type Wheeled%20Vehicle%20Pawn%20Soft%20Object%20Reference) (driver :type Character%20Soft%20Object%20Reference))
  (Variables|Default|SetVehicle (Utilities|ResolveSoftReference vehicle))
  (bind _output_get (Variables|Default|SetDriver (Utilities|ResolveSoftReference driver)))
  (Pawn|Possess (Pawn|GetController _output_get) (Variables|Default|GetVehicle)))