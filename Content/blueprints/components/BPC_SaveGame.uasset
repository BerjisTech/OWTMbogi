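; BPC_SaveGame is a component that manages the player's save data through an SG_PlayerData save object.
; On BeginPlay it loads the named slot if it exists, otherwise it creates a new save object.
; VehiclePossesed writes the possessed vehicle into the active vehicle field, resetting some of that record's other fields to defaults.
; Tick asynchronously saves the object to the slot every frame whenever it is valid.
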(event EventBeginPlay
  (bind _returnvalue (SaveGame|DoesSaveGameExist (Variables|Default|GetSlot%20Name)))
  (if _returnvalue
    (Utilities|LoadGame)
    (else
      (Utilities|CreateGame))))

(event EventTick
  (params (DeltaSeconds :type Float%20%28single-precision%29))
  (Utilities|SaveGame))

(event EventVehiclePossesed
  (params (possedVehicle :type Wheeled%20Vehicle%20Pawn%20Soft%20Object%20Reference))
  (Variables|/openWorldTemplate/blueprints/game_save/SG_PlayerData.SG_PlayerData_C|Setactivevehicle (Variables|Default|GetSG%20Player%20Data) (Utilities|Struct|MakeSTRUCT_PlayerVehicles 0 possedVehicle "None" 0.0 false "((\"engine\", 100.000000),(\"bumper\", 100.000000),(\"body\", 100.000000),(\"spolier\", 100.000000),(\"mirrors\", 100.000000),(\"wheelFR\", 100.000000),(\"wheelFL\", 0.000000),(\"wheelBR\", 0.000000),(\"wheelBL\", 0.000000))" "0.000000,0.000000,0.000000" "(name_2_38D6973243BB4D2EE21CB2932BD1B921=\"\",location_5_0560134B4B19CF6517C8B7B708788F57=(X=0.000000,Y=0.000000,Z=0.000000),hasGarage_8_CAAB9D58402A64923E2CBD849625BCC8=False,hasOffice_10_6E5E823C4763A7C05C68AD87DC6CC612=False,price_12_B276A79042F88185F416698B74BBD2EA=False,garageSize_14_A5A4CF2146331F525B147287B4A82D97=False,triggerMissions_18_4B1FF8E843557D01A2E253B96BA93E36=)")))