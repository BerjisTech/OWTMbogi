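; Player interaction component that lets a character board a nearby wheeled vehicle through Enhanced Input.
; On interact, it picks the nearest vehicle within range or spawns a base vehicle pawn by the player, then adds a vehicle interaction component to it.
; It loops moving the player toward the vehicle with tiny delays until close, then messages that component to possess it.
; Its own PossessVehicle event hands the vehicle's controller back to the driver.
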(event Input|EnhancedActionEvents|EnhancedInputActionIA_Interact
  (params (ActionValue :type Boolean) (ElapsedSeconds :type Float%20%28double-precision%29) (TriggeredSeconds :type Float%20%28double-precision%29) (InputAction :type Input%20Action%20Object%20Reference :default "/openWorldTemplate/blueprints/Input/Actions/IA_Interact.IA_Interact"))
  (bind _returnvalue (Components|GetOwner))
  (bind _returnvalue_2 (Transformation|GetActorTransform _returnvalue))
  (:Started
    (bind _outactors (Actor|GetAllActorsOfClass "/Script/ChaosVehicles.WheeledVehiclePawn"))
    (if (Utilities|Array|IsEmpty _outactors)
      (bind _returnvalue_3 (Game|SpawnActorfromClass "/openWorldTemplate/vehicles/blueprint/VehicleBasePawn.VehicleBasePawn_C" (Math|Transform|MakeTransform (+ (.location _returnvalue_2) 1e+02) (.rotation _returnvalue_2) (.scale _returnvalue_2)) "AdjustIfPossibleButAlwaysSpawn" "MultiplyWithRoot" 0 0 :!label _label))
      (Variables|Default|SetVehicle _returnvalue_3)
      (elif (< (.Distance (Actor|FindNearestActor (Transformation|GetActorLocation (Components|GetOwner)) _outactors)) (Variables|Default|GetnearestVehicleMaxDistanceAway))
        (Variables|Default|SetVehicle (.AsWheeled%20Vehicle%20Pawn (Utilities|Casting|CastToWheeledVehiclePawn (.ReturnValue (Actor|FindNearestActor (Transformation|GetActorLocation (Components|GetOwner)) _outactors)))))
        (else
          (goto _label))))
    (bind _returnvalue_4 (Utilities|AddInteractionComponent (Variables|Default|GetVehicle) "/openWorldTemplate/blueprints/components/BPC_VehicleInteraction.BPC_VehicleInteraction_C"))
    (Utilities|MovePlayertoLocation (Components|GetOwner) (Variables|Default|GetVehicle) :!label _label_2)
    (Utilities|FlowControl|Delay 0.0002)
    (if (< (.Distance (Actor|FindNearestActor (Transformation|GetActorLocation (Components|GetOwner)) _outactors)) (Variables|Default|GetminDistanceToPossesVehicle))
      (Class|BPIWorldInteraction|PossessVehicle(Message) _returnvalue_4 false false (Utilities|ResolveSoftReference (.AsWheeled%20Vehicle%20Pawn (Utilities|Casting|CastToWheeledVehiclePawn (.ReturnValue (Actor|FindNearestActor (Transformation|GetActorLocation (Components|GetOwner)) _outactors))))) (Utilities|ResolveSoftReference (.AsCharacter (Utilities|Casting|CastToCharacter (Components|GetOwner)))))
      (else
        (goto _label_2)))))

(event EventBeginPlay
  (Input|AddMappingContext (PlayerController|LocalPlayerSubsystems|GetEnhancedInputLocalPlayerSubsystem (Game|GetPlayerController 0)) "/openWorldTemplate/blueprints/Input/IMC_OWT.IMC_OWT" 1 "(bIgnoreAllPressedKeysUntilRelease=True,bForceImmediately=False,bNotifyUserSettings=False)"))

(event EventTick
  (params (DeltaSeconds :type Float%20%28single-precision%29)))

(event EventPossessVehicle
  (params (possess :type Boolean) (is_npc :type Boolean) (vehicle :type Wheeled%20Vehicle%20Pawn%20Soft%20Object%20Reference) (driver :type Character%20Soft%20Object%20Reference))
  (bind _output_get (Variables|Default|SetVehicle (Utilities|ResolveSoftReference vehicle)))
  (bind _output_get_2 (Variables|Default|SetDriver (Utilities|ResolveSoftReference driver)))
  (Pawn|Possess (Pawn|GetController _output_get) _output_get_2))