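; Common helper functions that snap a world location vertically onto the landscape.
; PlaceOnGround runs a long vertical multi line trace through the location via LineTraceForLandscape, against WorldStatic objects.
; The trace returns the first LandscapeStreamingProxy impact, printing names of other actors hit before it.
; Without a landscape hit it falls back to the last impact, or to the raised trace start when nothing is hit.
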(fn PlaceonGround
  (params (currentObjectLocation :type Vector))
  (bind _output_get (LocalVariables|SetoutHitLocation currentObjectLocation))
  (bind _array_element_impact_point (CallFunction|LineTraceforLandscape (+ _output_get "0.000000,0.000000,100000.000000") (+ _output_get "0.000000,0.000000,-1000000.000000")))
  (return _array_element_impact_point))

(fn LineTraceforLandscape
  (params (Start :type Vector) (End :type Vector :default "0.000000,0.000000,-1000000.000000"))
  (bind (_outhits _returnvalue) (Class|KismetSystemLibrary|LineTraceMultiforObjects 0 Start End (Utilities|Array|MakeArray "ObjectTypeQuery1") false 0 "None" true "(R=1.000000,G=0.000000,B=0.000000,A=0.246000)" "(R=0.000000,G=1.000000,B=0.000000,A=0.241000)"))
  (if _returnvalue
    (bind _array_element (Utilities|Array|ForEachLoopwithBreak _outhits :!label _label)
      (:LoopBody
        (LocalVariables|SetoutHitLocation (.impactpoint _array_element))
        (if (Class|GameplayStatics|ObjectIsA (.hitactor _array_element) "/Script/Landscape.LandscapeStreamingProxy")
          (goto _label Break)
          (else
            (Development|PrintString 0 (Utilities|GetDisplayName (.hitactor _array_element))))))
      (:Completed
        (return (LocalVariables|GetoutHitLocation))))
    (else
      (Development|PrintString 0 (Utilities|String|ToString(Boolean) _returnvalue))
      (return Start))))